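; BP_Ball1 is a short-lived physics ball actor built around a Sphere component.
; On BeginPlay it sets the sphere's angular velocity from its right, up and forward vectors, each multiplied by zero, so the initial spin is zero.
; Tick runs a five-second Delay and then destroys the actor, acting as a lifetime timer.
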(event `self.ReceiveBeginPlay`
  (bind _sphere (`self.Sphere`))
  (`PrimitiveComponent.SetPhysicsAngularVelocityInDegrees` _sphere (+ (* (`SceneComponent.GetRightVector` _sphere) (0.0 0.0 0.0)) (* (`SceneComponent.GetUpVector` _sphere) (0.0 0.0 0.0)) (* (`SceneComponent.GetForwardVector` _sphere) (0.0 0.0 0.0))) false "None"))

(event `self.ReceiveTick`
  (params (DeltaSeconds :type "Float (single-precision)"))
  (`KismetSystemLibrary.Delay` 5.0)
  (`self.K2_DestroyActor`))

(fn `UserConstructionScript`)